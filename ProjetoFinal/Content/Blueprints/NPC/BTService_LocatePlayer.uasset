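; Behavior Tree service that lets an NPC detect the player character within a search radius.
; Each tick it runs a multi-sphere trace for Pawn objects at the controlled pawn's location, with the radius read from the SearchRadius blackboard key.
; A hit that casts to BP_MainCharacter is written to the TargetActor key, which is cleared when none is found.
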(event `self.ReceiveTickAI`
  (params (OwnerController :type "AIController Object Reference") (ControlledPawn :type "Pawn Object Reference") (DeltaSeconds :type "Float (single-precision)"))
  (bind _returnvalue (`Actor.K2_GetActorLocation` ControlledPawn))
  (bind _as_bp_main_character (`self.As BP Main Character`))
  (bind _targetactor (`self.TargetActor`))
  (set `self.As BP Main Character` null)
  (bind (_outhits _returnvalue_2) (`KismetSystemLibrary.SphereTraceMultiForObjects` _returnvalue _returnvalue (`BTFunctionLibrary.GetBlackboardValueAsFloat` (`self.SearchRadius`)) (`|MakeArray` "ObjectTypeQuery3" :!type "EObjectTypeQuery Enum")))
  (if _returnvalue_2
    (for _array_element _outhits
      (bind _asbp_main_character (cast `/Game/Blueprints/Characters/BP_MainCharacter` (`.HitActor` (`GameplayStatics.BreakHitResult` _array_element))))
      (set `self.As BP Main Character` _asbp_main_character)))
  (`/Engine/EditorBlueprintResources/StandardMacros.IsValid` _as_bp_main_character
    (:`Is Valid`
      (`BTFunctionLibrary.SetBlackboardValueAsObject` _targetactor _as_bp_main_character))
    (:`Is Not Valid`
      (`BTFunctionLibrary.ClearBlackboardValue` _targetactor))))