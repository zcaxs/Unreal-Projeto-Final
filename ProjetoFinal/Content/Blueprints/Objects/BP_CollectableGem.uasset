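; BP_CollectableGem is the level-ending gem pickup that scores points and shows a win screen.
; On sphere overlap it casts the player pawn to BP_MainCharacter, adds a large bonus to PickUpCollectable, destroys itself and disables the character's input.
; The level name cached at BeginPlay picks the widget: BP_WinScreen for Level3, otherwise W_WinLevel with the score passed in.
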(event `self.ReceiveBeginPlay`
  (bind _returnvalue (`GameplayStatics.GetCurrentLevelName` true))
  (set `self.LevelName` (`KismetStringLibrary.Conv_StringToName` _returnvalue)))

(event `self.Sphere.OnComponentBeginOverlap`
  (params (OverlappedComponent :type "PrimitiveComponent Object Reference") (OtherActor :type "Actor Object Reference") (OtherComp :type "PrimitiveComponent Object Reference") (OtherBodyIndex :type Integer) (bFromSweep :type Boolean) (SweepResult :type "HitResult Structure (by ref)"))
  (bind _asbp_main_character (cast `/Game/Blueprints/Characters/BP_MainCharacter` (`GameplayStatics.GetPlayerCharacter` 0)))
  (bind _output_get (set `/Game/Blueprints/Characters/BP_MainCharacter.PickUpCollectable` (+ (`/Game/Blueprints/Characters/BP_MainCharacter.PickUpCollectable` _asbp_main_character) 1000) _asbp_main_character))
  (`self.K2_DestroyActor`)
  (`self.DisableInput` _asbp_main_character null)
  (if (== (`self.LevelName`) "Level3")
    (bind _returnvalue (`|CreateWidget` "/Game/Widgets/BP_WinScreen.BP_WinScreen_C"))
    (bind _output_get_2 (set `self.W_WinScreen` _returnvalue))
    (`UserWidget.AddToViewport` _output_get_2 0)
    (else
      (bind _returnvalue_2 (`|CreateWidget` "/Game/Widgets/W_WinLevel.W_WinLevel_C" (`GameplayStatics.GetPlayerController` 0) _output_get))
      (bind _output_get_3 (set `self.W_WinLevel` _returnvalue_2))
      (`UserWidget.AddToViewport` _output_get_3 0))))

(fn `UserConstructionScript`)