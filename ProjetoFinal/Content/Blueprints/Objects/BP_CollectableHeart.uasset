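; BP_CollectableHeart is a heart pickup that heals the main character on overlap.
; When its Sphere overlaps BP_MainCharacter below the hardcoded health cap, it adds one health and updates the gameplay widget's health display.
; At full health it adds bonus points to the character's PickUpCollectable value instead, and it destroys itself in both cases.
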(event `self.Sphere.OnComponentBeginOverlap`
  (params (OverlappedComponent :type "PrimitiveComponent Object Reference") (OtherActor :type "Actor Object Reference") (OtherComp :type "PrimitiveComponent Object Reference") (OtherBodyIndex :type Integer) (bFromSweep :type Boolean) (SweepResult :type "HitResult Structure (by ref)"))
  (bind _asbp_main_character (cast `/Game/Blueprints/Characters/BP_MainCharacter` OtherActor))
  (bind _currenthealth (`/Game/Blueprints/Characters/BP_MainCharacter.CurrentHealth` _asbp_main_character))
  (if (< _currenthealth 3)
    (bind _output_get (set `/Game/Blueprints/Characters/BP_MainCharacter.CurrentHealth` (+ _currenthealth 1) _asbp_main_character))
    (`/Game/Widgets/W_Gameplay.SetHealth` (`/Game/Blueprints/Characters/BP_MainCharacter.W_Gameplay` _asbp_main_character) _output_get 3)
    (`self.K2_DestroyActor`)
    (else
      (set `/Game/Blueprints/Characters/BP_MainCharacter.PickUpCollectable` (+ (`/Game/Blueprints/Characters/BP_MainCharacter.PickUpCollectable` _asbp_main_character) 500) _asbp_main_character)
      (`self.K2_DestroyActor`))))

(fn `UserConstructionScript`)