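; BP_InteractableSign is a world sign that shows a detail screen when the player interacts nearby.
; Sphere overlap toggles a proximity flag, outline overlay material and prompt widgets, with exit also removing the detail screen.
; BeginPlay binds to the player controller's E-key dispatcher.
; Interact creates the detail widget with the sign's texture index, then reuses that instance on later views.
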(event `self.Sphere.OnComponentBeginOverlap`
  (params (OverlappedComponent :type "PrimitiveComponent Object Reference") (OtherActor :type "Actor Object Reference") (OtherComp :type "PrimitiveComponent Object Reference") (OtherBodyIndex :type Integer) (bFromSweep :type Boolean) (SweepResult :type "HitResult Structure (by ref)"))
  (set `self.IsPlayerNearby?` true)
  (`MeshComponent.SetOverlayMaterial` (`self.StaticMesh`) "/Game/Materials/Interactions/M_Outline_Ins.M_Outline_Ins")
  (`SceneComponent.SetVisibility` (`self.InteractableWidget`) true false)
  (`SceneComponent.SetVisibility` (`self.InteractWidget`) true false))

(event `self.Sphere.OnComponentEndOverlap`
  (params (OverlappedComponent :type "PrimitiveComponent Object Reference") (OtherActor :type "Actor Object Reference") (OtherComp :type "PrimitiveComponent Object Reference") (OtherBodyIndex :type Integer))
  (bind _output_get (set `self.IsPlayerNearby?` false))
  (if (not _output_get)
    (`Widget.RemoveFromParent` (`self.W_SignDetails`))
    (`MeshComponent.SetOverlayMaterial` (`self.StaticMesh`) null)
    (`SceneComponent.SetVisibility` (`self.InteractableWidget`) false false)
    (`SceneComponent.SetVisibility` (`self.InteractWidget`) false false)))

(event `/Game/Blueprints/Interfaces/BPI_Interactable.Interact`
  (bind _w_signdetails (`self.W_SignDetails`))
  (if (`self.IsPlayerNearby?`)
    (`/Engine/EditorBlueprintResources/StandardMacros.IsValid` _w_signdetails
      (:`Is Valid`
        (`UserWidget.AddToViewport` _w_signdetails 0))
      (:`Is Not Valid`
        (bind _returnvalue (`|CreateWidget` "/Game/Widgets/W_SignDetails.W_SignDetails_C" (`GameplayStatics.GetPlayerController` 0) (`self.SignTextureIndex`)))
        (bind _output_get (set `self.W_SignDetails` _returnvalue))
        (`UserWidget.AddToViewport` _output_get 0)))))

(event `self.ReceiveBeginPlay`
  (bind _asbp_main_player_controller (cast `/Game/Blueprints/Controllers/BP_MainPlayerController` (`GameplayStatics.GetPlayerController` 0)))
  (add `/Game/Blueprints/Controllers/BP_MainPlayerController.OnKeyEPressed` _asbp_main_player_controller (`|CreateDelegate` :!event `Interact`)))

(fn `UserConstructionScript`)