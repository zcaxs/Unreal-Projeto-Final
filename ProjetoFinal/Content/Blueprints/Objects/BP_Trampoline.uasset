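; BP_Trampoline is a trampoline object that launches the player character and re-enables its dash.
; On BeginPlay it caches player 0's character as BP_MainCharacter.
; When anything begins overlapping its Box while IsOnTrampoline is true, it launches that cached character along configurable X, Y and force values, overriding existing velocity, and sets CanDash.
; The overlapping actor is never checked, and IsOnTrampoline is not set within this Blueprint.
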(event `self.ReceiveBeginPlay`
  (bind _asbp_main_character (cast `/Game/Blueprints/Characters/BP_MainCharacter` (`GameplayStatics.GetPlayerCharacter` 0)))
  (set `self.As BP Main Character` _asbp_main_character))

(event `self.Box.OnComponentBeginOverlap`
  (params (OverlappedComponent :type "PrimitiveComponent Object Reference") (OtherActor :type "Actor Object Reference") (OtherComp :type "PrimitiveComponent Object Reference") (OtherBodyIndex :type Integer) (bFromSweep :type Boolean) (SweepResult :type "HitResult Structure (by ref)"))
  (bind _as_bp_main_character (`self.As BP Main Character`))
  (if (`self.IsOnTrampoline?`)
    (`Character.LaunchCharacter` _as_bp_main_character (+ (0.0 0.0 0.0) (`KismetMathLibrary.MakeVector` (`self.TrampolineDirectionX`) (`self.TrampolineDirectionY`) (`self.TrampolineForce`))) true true)
    (set `/Game/Blueprints/Characters/BP_MainCharacter.CanDash?` true _as_bp_main_character)))

(fn `UserConstructionScript`)