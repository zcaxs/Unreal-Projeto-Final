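; BP_Spikes is a hazard that costs the main character one health point and returns it to a respawn point.
; It caches the player character on BeginPlay, and any overlap with its box acts on that cached reference without checking the overlapping actor.
; The overlap disables input, plays the death montage, waits for its duration, then moves the player to the first actor tagged Respawn and re-enables input.
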(event `self.ReceiveBeginPlay`
  (bind _asbp_main_character (cast `/Game/Blueprints/Characters/BP_MainCharacter` (`GameplayStatics.GetPlayerCharacter` 0)))
  (set `self.As BP Main Character` _asbp_main_character))

(event `self.Box.OnComponentBeginOverlap`
  (params (OverlappedComponent :type "PrimitiveComponent Object Reference") (OtherActor :type "Actor Object Reference") (OtherComp :type "PrimitiveComponent Object Reference") (OtherBodyIndex :type Integer) (bFromSweep :type Boolean) (SweepResult :type "HitResult Structure (by ref)"))
  (bind _as_bp_main_character (`self.As BP Main Character`))
  (`/Game/Widgets/W_Gameplay.SetHealth` (`/Game/Blueprints/Characters/BP_MainCharacter.W_Gameplay` _as_bp_main_character) (- (`/Game/Blueprints/Characters/BP_MainCharacter.CurrentHealth` _as_bp_main_character) 1) (`/Game/Blueprints/Characters/BP_MainCharacter.MaxHealth` _as_bp_main_character))
  (`self.DisableInput` _as_bp_main_character null)
  (bind _returnvalue (`Character.PlayAnimMontage` _as_bp_main_character "/Game/Animations/Char_Die_Montage.Char_Die_Montage" 1.0 "None"))
  (`KismetSystemLibrary.Delay` _returnvalue)
  (bind _outactors (`GameplayStatics.GetAllActorsWithTag` "Respawn"))
  (`self.K2_SetActorLocation` _as_bp_main_character (`self.K2_GetActorLocation` (`|GetArrayItem` _outactors)) false false)
  (`self.EnableInput` _as_bp_main_character null))

(fn `UserConstructionScript`)