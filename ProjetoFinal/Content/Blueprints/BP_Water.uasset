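; BP_Water is a water hazard that costs the player one health point and sends them back to a fixed location.
; Any overlap with WaterCollision updates the cached main character's health widget, disables input, then teleports the character after a short delay, without checking what overlapped.
; Input returns if health remains; otherwise movement stops and the Game Over widget replaces the gameplay HUD with UI-only input.
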(event `self.ReceiveBeginPlay`
  (bind _asbp_main_character (cast `/Game/Blueprints/Characters/BP_MainCharacter` (`GameplayStatics.GetPlayerCharacter` 0)))
  (set `self.As BP Main Character` _asbp_main_character))

(event `self.WaterCollision.OnComponentBeginOverlap`
  (params (OverlappedComponent :type "PrimitiveComponent Object Reference") (OtherActor :type "Actor Object Reference") (OtherComp :type "PrimitiveComponent Object Reference") (OtherBodyIndex :type Integer) (bFromSweep :type Boolean) (SweepResult :type "HitResult Structure (by ref)"))
  (bind _returnvalue (`GameplayStatics.GetPlayerController` 0))
  (bind _as_bp_main_character (`self.As BP Main Character`))
  (bind _w_gameplay (`/Game/Blueprints/Characters/BP_MainCharacter.W_Gameplay` _as_bp_main_character))
  (bind _currenthealth (`/Game/Blueprints/Characters/BP_MainCharacter.CurrentHealth` _as_bp_main_character))
  (set `/Game/Blueprints/Characters/BP_MainCharacter.CurrentHealth` (`KismetMathLibrary.Max` (- _currenthealth 1)) _as_bp_main_character)
  (`/Game/Widgets/W_Gameplay.SetHealth` _w_gameplay _currenthealth (`/Game/Blueprints/Characters/BP_MainCharacter.MaxHealth` _as_bp_main_character))
  (`self.DisableInput` _as_bp_main_character null)
  (`KismetSystemLibrary.Delay` 0.5)
  (`self.K2_SetActorRotation` :`self` _as_bp_main_character)
  (`self.K2_SetActorLocation` _as_bp_main_character (-4000.0 0.0 230.0) false false)
  (if (<= _currenthealth 0)
    (`CharacterMovementComponent.DisableMovement` (`Character.CharacterMovement` _as_bp_main_character))
    (bind _returnvalue_2 (`|CreateWidget` "/Game/Widgets/W_GameOver.W_GameOver_C"))
    (bind _output_get (set `self.W_GameOver` _returnvalue_2))
    (`UserWidget.AddToViewport` _output_get 0)
    (`Widget.RemoveFromParent` _w_gameplay)
    (`WidgetBlueprintLibrary.SetInputMode_UIOnlyEx` _returnvalue null)
    (set `PlayerController.bShowMouseCursor` true _returnvalue)
    (else
      (`self.EnableInput` _as_bp_main_character null))))

(fn `UserConstructionScript`)