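; BP_MainCharacter is the player character, handling Enhanced Input look, move and jump.
; On BeginPlay it sets game-only input, adds the W_Gameplay widget to the viewport and fills CurrentHealth from MaxHealth.
; Move applies input along control-rotation axes, with forward flattened to yaw.
; An IsJumping flag set on jump and cleared shortly after landing blocks immediate re-jumps.
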(event `self.ReceiveBeginPlay`
  (`WidgetBlueprintLibrary.SetInputMode_GameOnly` (`GameplayStatics.GetPlayerController` 0))
  (bind _returnvalue (`|CreateWidget` "/Game/Widgets/W_Gameplay.W_Gameplay_C"))
  (bind _output_get (set `self.W_Gameplay` _returnvalue))
  (`UserWidget.AddToViewport` _output_get 0)
  (set `self.CurrentHealth` (`self.MaxHealth`)))

(event `EnhancedInput|/Game/Inputs/InputMotions/IA_Look`
  (params (ActionValue :type "Vector2D Structure") (ElapsedSeconds :type "Float (double-precision)") (TriggeredSeconds :type "Float (double-precision)") (InputAction :type "InputAction Object Reference" :default "/Game/Inputs/InputMotions/IA_Look.IA_Look"))
  (:`Triggered`
    (`self.AddControllerYawInput` ActionValue_X)
    (`self.AddControllerPitchInput` ActionValue_Y)))

(event `EnhancedInput|/Game/Inputs/InputMotions/IA_Move`
  (params (ActionValue :type "Vector2D Structure") (ElapsedSeconds :type "Float (double-precision)") (TriggeredSeconds :type "Float (double-precision)") (InputAction :type "InputAction Object Reference" :default "/Game/Inputs/InputMotions/IA_Move.IA_Move"))
  (:`Triggered`
    (`self.Move` ActionValue_X ActionValue_Y)))

(event `EnhancedInput|/Game/Inputs/InputMotions/IA_Jump`
  (params (ActionValue :type Boolean) (ElapsedSeconds :type "Float (double-precision)") (TriggeredSeconds :type "Float (double-precision)") (InputAction :type "InputAction Object Reference" :default "/Game/Inputs/InputMotions/IA_Jump.IA_Jump"))
  (:`Triggered`
    (if (not (`self.IsJumping?`))
      (`self.Jump`)))
  (:`Canceled`
    (`self.StopJumping` :!label _label))
  (:`Completed`
    (goto _label)))

(event `self.OnJumped`
  (set `self.IsJumping?` true))

(event `self.OnLanded`
  (params (Hit :type "HitResult Structure (by ref)"))
  (`KismetSystemLibrary.Delay` 0.2)
  (set `self.IsJumping?` false))

(fn `Move`
  (params (InputPin :type "Float (double-precision)") (InputPin2 :type "Float (double-precision)"))
  (bind (_returnvalue_roll _returnvalue_pitch _returnvalue_yaw) (`KismetMathLibrary.BreakRotator` (`self.GetControlRotation`)))
  (bind (_returnvalue_roll_2 _returnvalue_pitch_2 _returnvalue_yaw_2) (`KismetMathLibrary.BreakRotator` (`self.GetControlRotation`)))
  (`self.AddMovementInput` (`KismetMathLibrary.GetRightVector` (`KismetMathLibrary.MakeRotator` _returnvalue_roll_2 0.0 _returnvalue_yaw_2)) InputPin)
  (`self.AddMovementInput` (`KismetMathLibrary.GetForwardVector` (`KismetMathLibrary.MakeRotator` 0.0 0.0 _returnvalue_yaw)) InputPin2))

(fn `UserConstructionScript`)